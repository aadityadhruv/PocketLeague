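; Spawner actor that places a BP_Boost pickup 50 units above its location on BeginPlay and respawns one on request.
; TriggerBoostSpawn sets the NeedToSpawn flag, which Tick polls and clears before waiting three seconds and calling SpawnBoost again.
; Each spawned boost gets the spawner as its Owner; nothing in this Blueprint calls the trigger itself.
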(event `self.ReceiveBeginPlay`
  (`self.SpawnBoost`))

(event `self.ReceiveTick`
  (params (DeltaSeconds :type "Float (single-precision)"))
  (if (`self.needToSpawn`)
    (set `self.needToSpawn` false)
    (`KismetSystemLibrary.Delay` 3.0)
    (`self.SpawnBoost`)))

(fn `SpawnBoost`
  (`|SpawnActorFromClass` "/Game/Boost/BP_Boost.BP_Boost_C" (`KismetMathLibrary.Conv_VectorToTransform` (+ (`self.K2_GetActorLocation`) (0.0 0.0 50.0))) "Undefined" "OverrideRootScale" self null))

(fn `Trigger Boost Spawn`
  (set `self.needToSpawn` true))

(fn `UserConstructionScript`)