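; BP_Goal is a team goal that detects a BP_Ball overlap and runs the scoring sequence.
; A goal plays a hit effect, destroys the ball, updates BP_ScoreHandler using IsBlue, and blasts all BP_Car and BP_Poncho actors outward and upward from the goal.
; After a short delay it resets those actors' locations and spawns a new ball.
; IsBlue also applies the M_Goal material to the walls at BeginPlay.
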(event `self.ReceiveBeginPlay`
  (if (`self.isBlue`)
    (`PrimitiveComponent.SetMaterial` (`self.wallRight`) 0 "/Game/Goal/M_Goal.M_Goal")
    (`PrimitiveComponent.SetMaterial` (`self.wallLeft`) 0 "/Game/Goal/M_Goal.M_Goal")
    (`PrimitiveComponent.SetMaterial` (`self.wallBack`) 0 "/Game/Goal/M_Goal.M_Goal")
    (`PrimitiveComponent.SetMaterial` (`self.wallTop`) 0 "/Game/Goal/M_Goal.M_Goal")))

(event `self.ReceiveActorBeginOverlap`
  (params (OtherActor :type "Actor Object Reference"))
  (bind _asbp_ball (cast `/Game/Ball/BP_Ball` OtherActor))
  (`GameplayStatics.SpawnEmitterAtLocation` "/Game/FXVarietyPack/Particles/P_ky_waterBallHit.P_ky_waterBallHit" (`SceneComponent.K2_GetComponentLocation` (`/Game/Ball/BP_Ball.Sphere` _asbp_ball)) (struct) (10.0 10.0 10.0))
  (`self.K2_DestroyActor` _asbp_ball)
  (bind _returnvalue (`GameplayStatics.GetActorOfClass` "/Game/GameHandler/BP_ScoreHandler.BP_ScoreHandler_C"))
  (`/Game/GameHandler/BP_ScoreHandler.UpdateScore` _returnvalue (`self.isBlue`))
  (`self.ThrowPlayers`)
  (`KismetSystemLibrary.Delay` 3.0)
  (`self.RespawnAll`)
  (`|SpawnActorFromClass` "/Game/Ball/BP_Ball.BP_Ball_C" (`KismetMathLibrary.MakeTransform` (0.0 0.0 150.0)) "Undefined" "OverrideRootScale" null null))

(fn `AddForceToComponent`
  (params (Mesh :type "PrimitiveComponent Object Reference") (location :type "Vector Structure"))
  (`PrimitiveComponent.AddForce` Mesh (+ (* (* (`KismetMathLibrary.Normal` (- location (`self.K2_GetActorLocation`))) 2000000000.0) (1.0 1.0 0.0)) (0.0 0.0 1000000000.0)) "None" false))

(fn `RespawnAll`
  (bind _outactors (`GameplayStatics.GetAllActorsOfClass` "/Game/VehicleBP/Sedan/BP_Car.BP_Car_C"))
  (for _array_element _outactors
    (`/Game/VehicleBP/Sedan/BP_Car.Reset Location` _array_element))
  (bind _outactors_2 (`GameplayStatics.GetAllActorsOfClass` "/Game/Bot/BP_Poncho.BP_Poncho_C"))
  (for _array_element_2 _outactors_2
    (`/Game/Bot/BP_Poncho.ResetLocation` _array_element_2)))

(fn `ThrowPlayers`
  (bind _outactors (`GameplayStatics.GetAllActorsOfClass` "/Game/VehicleBP/Sedan/BP_Car.BP_Car_C"))
  (for _array_element _outactors
    (`self.AddForceToComponent` (`WheeledVehicle.Mesh` _array_element) (`self.K2_GetActorLocation` _array_element)))
  (bind _outactors_2 (`GameplayStatics.GetAllActorsOfClass` "/Game/Bot/BP_Poncho.BP_Poncho_C"))
  (for _array_element_2 _outactors_2
    (`self.AddForceToComponent` (`WheeledVehicle.Mesh` _array_element_2) (`self.K2_GetActorLocation` _array_element_2))))

(fn `UserConstructionScript`)