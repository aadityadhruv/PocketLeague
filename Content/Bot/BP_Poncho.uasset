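; BP_Poncho is a bot vehicle that drives at full throttle toward the BP_Ball actor.
; Each Tick, GetSteering maps the unnormalized yaw difference to the ball into clamped steering input, with debug line and prints.
; Boost spends a charge to add capped forward velocity with shockwave effects, and dodge plays an animation with its force push disconnected.
; Boost, dodge and the angle-to-ball helper are not called within this Blueprint.
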(event `self.ReceiveBeginPlay`)

(event `self.ReceiveTick`
  (params (DeltaSeconds :type "Float (single-precision)"))
  ;[1 1 1] Movement and Steering
  (`|ExecutionSequence`
    (:`then_0`
      (bind _axis (`self.GetSteering`))
      (`WheeledVehicleMovementComponent.SetSteeringInput` (`self.VehicleMovement`) _axis))
    (:`then_1`
      (`WheeledVehicleMovementComponent.SetThrottleInput` (`self.VehicleMovement`) 1.0))))

(fn `ActionBoost`
  ;[1 1 1] Boosting
  (if (> (`self.boostAmount`) 0)
    (bind _returnvalue (`PrimitiveComponent.GetPhysicsLinearVelocity` (`self.Mesh`) "None"))
    (`PrimitiveComponent.SetPhysicsLinearVelocity` (`self.Mesh`) (`KismetMathLibrary.ClampVectorSize` (+ _returnvalue (* (`self.GetActorForwardVector`) 100.0)) 0.0 (`self.maxSpeed`)) false "None")
    (`/Engine/EditorBlueprintResources/StandardMacros.DecrementInt` (`self.boostAmount`)
      (:`  `
        (`GameplayStatics.SpawnEmitterAttached` "/Game/FXVarietyPack/Particles/P_ky_shotShockwave.P_ky_shotShockwave" (`self.leftBoost`))
        (`GameplayStatics.SpawnEmitterAttached` "/Game/FXVarietyPack/Particles/P_ky_shotShockwave.P_ky_shotShockwave" (`self.rightBoost`))))))

(fn `ActionDodge`
  (`SkeletalMeshComponent.SetPhysicsBlendWeight` (`self.Mesh`) 0.2)
  (`SkeletalMeshComponent.PlayAnimation` (`self.Mesh`) "/Game/VehicleBP/Sedan/Anims/Small/working_dodge_small_Anim.working_dodge_small_Anim" false))

(fn `AngleBetweenVectors`
  (params (VecA :type "Vector Structure") (VecB :type "Vector Structure"))
  (returns (angle :type "Float (double-precision)"))
  (return (`KismetMathLibrary.DegAcos` (`KismetMathLibrary.Dot_VectorVector` (`KismetMathLibrary.Normal` VecA) (`KismetMathLibrary.Normal` VecB)))))

(fn `GetAngleToBall`
  (params (ballRef :type "/Game/Ball/BP_Ball Object Reference"))
  (returns (angle :type "Float (double-precision)"))
  (bind _angle (`self.AngleBetweenVectors` (`self.GetActorForwardVector`) (- (* (`self.K2_GetActorLocation` ballRef) (1.0 1.0 0.0)) (* (`self.K2_GetActorLocation`) (1.0 1.0 0.0)))))
  (return _angle))

(fn `GetSteering`
  (returns (axis :type "Float (double-precision)"))
  (bind (_returnvalue_roll _returnvalue_pitch _returnvalue_yaw) (`KismetMathLibrary.BreakRotator` (`self.K2_GetActorRotation`)))
  (bind _returnvalue (`self.K2_GetActorLocation`))
  (bind _returnvalue_2 (`GameplayStatics.GetActorOfClass` "/Game/Ball/BP_Ball.BP_Ball_C"))
  (`/Engine/EditorBlueprintResources/StandardMacros.IsValid` _returnvalue_2
    (:`Is Valid`
      (bind _returnvalue_3 (`SceneComponent.K2_GetComponentLocation` (`/Game/Ball/BP_Ball.Sphere` _returnvalue_2)))
      (`KismetSystemLibrary.DrawDebugLine` _returnvalue _returnvalue_3)
      (`KismetSystemLibrary.PrintString` (`KismetStringLibrary.Conv_DoubleToString` _returnvalue_yaw))
      (bind (_returnvalue_roll_2 _returnvalue_pitch_2 _returnvalue_yaw_2) (`KismetMathLibrary.BreakRotator` (`KismetMathLibrary.FindLookAtRotation` _returnvalue _returnvalue_3)))
      (`KismetSystemLibrary.PrintString` (`KismetStringLibrary.Conv_DoubleToString` _returnvalue_yaw_2))
      (return (`KismetMathLibrary.MapRangeClamped` (- _returnvalue_yaw_2 _returnvalue_yaw) -90.0 90.0 -1.0 1.0)))
    (:`Is Not Valid`
      (return 0.0))))

(fn `Update Boost`
  (params (boostGained :type Integer))
  (returns (didCollect :type Boolean))
  (if (< (`self.boostAmount`) (`self.maxBoost`))
    (set `self.boostAmount` (`KismetMathLibrary.Clamp` (+ (`self.boostAmount`) boostGained) 0 (`self.maxBoost`)))
    (return true)
    (else
      (return false))))

(fn `UserConstructionScript`)