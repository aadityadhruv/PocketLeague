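; BP_ClockHandler is the match countdown timer for a car game, ending the game when a set Duration runs out.
; It records a start time on BeginPlay, then each Tick computes the truncated seconds left and pushes it to every BP_Car's HUD clock.
; When time expires it pauses the game and sets IsGameOver on all cars, finding them through GetAllActorsOfClass every tick.
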(event `self.ReceiveBeginPlay`
  (set `self.startTime` (`self.GetGameTimeSinceCreation`)))

(event `self.ReceiveTick`
  (params (DeltaSeconds :type "Float (single-precision)"))
  (bind _returnvalue (- (`self.GetGameTimeSinceCreation`) (`self.startTime`)))
  (`self.UpdateTimeForPlayers` (`KismetMathLibrary.FTrunc` (- (`self.duration`) _returnvalue)))
  (if (>= _returnvalue (`self.duration`))
    (`GameplayStatics.SetGamePaused` true)
    (bind _outactors (`GameplayStatics.GetAllActorsOfClass` "/Game/VehicleBP/Sedan/BP_Car.BP_Car_C"))
    (for _array_element _outactors
      (set `/Game/VehicleBP/Sedan/BP_Car.isGameOver` true _array_element))))

(fn `UpdateTimeForPlayers`
  (params (timeLeft :type Integer))
  (bind _outactors (`GameplayStatics.GetAllActorsOfClass` "/Game/VehicleBP/Sedan/BP_Car.BP_Car_C"))
  (for _array_element _outactors
    (`/Game/VehicleBP/Sedan/WBP_HUD.UpdateClockTime` (`/Game/VehicleBP/Sedan/BP_Car.HUD` _array_element) timeLeft)))

(fn `UserConstructionScript`)