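; BP_ScoreHandler is an actor that tracks the Orange and Blue team scores and shows them on car HUDs.
; UpdateScore takes IsBlue and increments the opposite team's score (true adds to Orange, false to Blue), then pushes both totals to every BP_Car's HUD.
; Tick also repeats that all-car lookup and HUD push every frame.
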(event `self.ReceiveTick`
  (params (DeltaSeconds :type "Float (single-precision)"))
  (bind _outactors (`GameplayStatics.GetAllActorsOfClass` "/Game/VehicleBP/Sedan/BP_Car.BP_Car_C"))
  (for _array_element _outactors
    (`/Game/VehicleBP/Sedan/WBP_HUD.UpdateScore` (`/Game/VehicleBP/Sedan/BP_Car.HUD` _array_element) (`self.orangeScore`) (`self.blueScore`))))

(fn `UpdateScore`
  (params (isBlue :type Boolean))
  (if isBlue
    (`/Engine/EditorBlueprintResources/StandardMacros.IncrementInt` (`self.orangeScore`)
      (:`  `
        _))
    (else
      (`/Engine/EditorBlueprintResources/StandardMacros.IncrementInt` (`self.blueScore`)
        (:`  `
          _))))
  (bind _outactors (`GameplayStatics.GetAllActorsOfClass` "/Game/VehicleBP/Sedan/BP_Car.BP_Car_C"))
  (for _array_element _outactors
    (`/Game/VehicleBP/Sedan/WBP_HUD.UpdateScore` (`/Game/VehicleBP/Sedan/BP_Car.HUD` _array_element) (`self.orangeScore`) (`self.blueScore`))))

(fn `UserConstructionScript`)